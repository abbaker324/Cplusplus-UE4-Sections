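; Openable door actor that swings open and closed in response to OpenDoor OnOpen and OnClose events.
; BeginPlay stores the initial rotation, and the Door_Swing timeline combines its OpenAngle yaw with that rotation each update.
; Opening plays the timeline forward and closing reverses it.
; A Sound Timing event track on the timeline spawns the doorlock sound at the door's location.
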(event `self.ReceiveBeginPlay`
  (set `self.Initial Rotation` (`self.K2_GetActorRotation`)))

(event `self.OpenDoor.OnOpen`
  (bind (_direction _openangle) (`Timeline|Door_Swing` :!label _label)
    (:`Update`
      (`self.SetActorRotation` (`KismetMathLibrary.ComposeRotators` (`KismetMathLibrary.MakeRotator` 0.0 0.0 _openangle) (`self.Initial Rotation`))))
    (:`Sound Timing`
      (`GameplayStatics.SpawnSoundAtLocation` "/Game/door-lock_Cue.door-lock_Cue" (`self.K2_GetActorLocation`)))))

(event `self.OpenDoor.OnClose`
  (goto _label :!via `Reverse`))

(fn `UserConstructionScript`)